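; AI tank enemy that takes damage, explodes at zero health and notifies a health widget.
; Functions aim the turret at the player or along velocity, rotate the base, line-trace for aim and pick navigable points near the player.
; Fire spawns a rocket and calls a dispatcher meant to trigger a delayed reload.
; BeginPlay and Tick are empty, leaving the widget lookup and reload binding disconnected; no live graph calls the helpers.
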(event `self.ReceiveBeginPlay`)

(event `CustomEvent`
  (`KismetSystemLibrary.Delay` 0.5)
  (set `self.CanFire` true))

(event `self.ReceiveTick`
  (params (DeltaSeconds :type "Float (single-precision)")))

(event `self.ReceiveAnyDamage`
  (params (Damage :type "Float (single-precision)") (DamageType :type "DamageType Object Reference") (InstigatedBy :type "Controller Object Reference") (DamageCauser :type "Actor Object Reference"))
  (bind (_returnvalue_location _returnvalue_rotation) (`KismetMathLibrary.BreakTransform` (`self.GetTransform`)))
  (bind _output_get (set `self.Heaht` (- (`self.Heaht`) Damage)))
  (if (<= _output_get 0.0)
    (`GameplayStatics.PlaySoundAtLocation` "/Game/Tank/Rocket/mixkit-gun-explosion-with-long-echo-1700.mixkit-gun-explosion-with-long-echo-1700" _returnvalue_location (struct) 5.0 2.0 0.1 null null null null)
    (`self.K2_DestroyActor`)
    (`GameplayStatics.SpawnEmitterAtLocation` null _returnvalue_location _returnvalue_rotation (1.5 1.5 1.5))
    (`/Game/Tank/AI/WB_Health.vurdu` (`self.NewVar`))))

(fn `BP_AItATLUS_AutoGenFunc`)

(fn `Fire`
  (bind (_returnvalue_location _returnvalue_rotation) (`KismetMathLibrary.BreakTransform` (`SceneComponent.K2_GetComponentToWorld` (`self.Muzzle`))))
  (bind (_returnvalue_location_2 _returnvalue_rotation_2) (`KismetMathLibrary.BreakTransform` (`SceneComponent.K2_GetComponentToWorld` (`self.Muzzle`))))
  (if (`self.CanFire`)
    (`GameplayStatics.SpawnEmitterAtLocation` null _returnvalue_location_2 _returnvalue_rotation_2 (0.15 0.15 0.15))
    (`|SpawnActorFromClass` "/Game/Tank/Rocket/BP_Rocket.BP_Rocket_C" (`KismetMathLibrary.MakeTransform` _returnvalue_location _returnvalue_rotation (0.5 0.5 0.5)) "AdjustIfPossibleButAlwaysSpawn" "MultiplyWithRoot" null null)
    (set `self.CanFire` false)
    (`self.vurar`)))

(fn `GetRandomLoc`
  (returns (`Random Location` :type "Vector Structure"))
  (bind _randomlocation (`NavigationSystemV1.K2_GetRandomLocationInNavigableRadius` (`self.K2_GetActorLocation` (`GameplayStatics.GetPlayerPawn` 0)) 3000.0 null null :!label _label))
  (if (<= (`KismetMathLibrary.Vector_Distance` _randomlocation (`self.K2_GetActorLocation` (`GameplayStatics.GetPlayerPawn` 0))) 2000.0)
    (return _randomlocation)
    (else
      (goto _label))))

(fn `isAim`
  (returns (Looking :type Boolean))
  (bind _muzzle (`self.Muzzle`))
  (bind _returnvalue (`SceneComponent.K2_GetComponentLocation` _muzzle))
  (bind _outhit (`KismetSystemLibrary.LineTraceSingle` _returnvalue (+ _returnvalue (* (`KismetMathLibrary.GetForwardVector` (`SceneComponent.K2_GetComponentRotation` _muzzle)) 1500)) "TraceTypeQuery1"))
  (return (== (`.HitActor` (`GameplayStatics.BreakHitResult` _outhit)) (`GameplayStatics.GetPlayerPawn` 0))))

(fn `Rotate to Player`
  (`SceneComponent.K2_SetWorldRotation` (`self.Turret`) (`KismetMathLibrary.MakeRotator` 0.0 0.0 (- (.yaw (`KismetMathLibrary.FindLookAtRotation` (`SceneComponent.K2_GetComponentLocation` (`self.Turret`)) (`self.K2_GetActorLocation` (`GameplayStatics.GetPlayerPawn` 0)))) 90.0)) false false))

(fn `RotateBase`
  (`SceneComponent.K2_AddWorldRotation` (`self.Base`) (`KismetMathLibrary.MakeRotator` 0.0 0.0 (/ (`KismetMathLibrary.Dot_VectorVector` (`self.GetVelocity`) (`SceneComponent.GetRightVector` (`self.Arrow`))) 100.0)) false false))

(fn `TransformLocation`
  (params (Location :type "Vector Structure"))
  (returns (`Real Worl` :type "Vector Structure"))
  (return (`KismetMathLibrary.TransformLocation` (`self.GetTransform`) Location)))

(fn `Turret Rotate`
  (bind (_returnvalue_roll _returnvalue_pitch _returnvalue_yaw) (`KismetMathLibrary.BreakRotator` (`KismetMathLibrary.MakeRotFromX` (`KismetMathLibrary.Normal` (`self.GetVelocity`)))))
  (`SceneComponent.K2_SetRelativeRotation` (`self.Turret`) (`KismetMathLibrary.MakeRotator` 0.0 0.0 _returnvalue_yaw) false false))

(fn `UserConstructionScript`)