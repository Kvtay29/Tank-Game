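; AI controller for tanks that runs a behavior tree and blackboard on possess and reacts to sight and hearing.
; Perception updates pass each actor through CanSenseActor, which matches its last stimuli to a sense class.
; Sight switches the blackboard Stat enum; hearing, when nothing is seen, stores InvestigateLoc and sets another state.
; Losing sight only clears the Seeing flag, and the Player key setup is disconnected.
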(event `self.ReceivePossess`
  (params (PossessedPawn :type "Pawn Object Reference"))
  (`self.RunBehaviorTree` "/Game/Tank/AI/BT.BT")
  (bind _blackboardcomponent (`self.UseBlackboard` "/Game/Tank/AI/BB.BB"))
  (bind _output_get (set `self.Blackboard Component` _blackboardcomponent)))

(event `self.ReceiveTick`
  (params (DeltaSeconds :type "Float (single-precision)")))

(event `self.AIPerception.OnPerceptionUpdated`
  (params (UpdatedActors :type "Array of Actor Object Reference (by ref)"))
  (for _array_element UpdatedActors
    (`|ExecutionSequence`
      (:`then_0`
        (bind (_sensed _stimus) (`self.Can Sense Actor` _array_element "NewEnumerator0"))
        (if _sensed
          (set `self.Seeing` true)
          (`self.On See` _stimus)
          (else
            (set `self.Seeing` false))))
      (:`then_1`
        (bind (_sensed_2 _stimus_2) (`self.Can Sense Actor` _array_element "NewEnumerator2"))
        (if _sensed_2
          (if (not (`self.Seeing`))
            (`self.On Hearing` _stimus_2)))))))

(fn `Can Sense Actor`
  (params (Actor :type "Actor Object Reference") (Sense :type "/Game/Tank/AI/Enum/E_Sense Enum" :default "NewEnumerator3"))
  (returns (Sensed :type Boolean) (Stimus :type "AIStimulus Structure"))
  (bind _info (`AIPerceptionComponent.GetActorsPerception` (`self.AIPerception`) Actor))
  (for _array_element (`.LastSensedStimuli` (break `ActorPerceptionBlueprintInfo` _info))
    (bind _returnvalue (`AIPerceptionSystem.GetSenseClassForStimulus` _array_element))
    (if (== _returnvalue (select `/Game/Tank/AI/Enum/E_Sense` Sense :`NewEnumerator0` "/Script/AIModule.AISense_Sight" :`NewEnumerator1` "/Script/AIModule.AISense_Damage" :`NewEnumerator2` "/Script/AIModule.AISense_Hearing" :!type "Object Class Reference"))
      (return (`.bSuccessfullySensed` (break `AIStimulus` _array_element)) _array_element))))

(fn `On Hearing`
  (params (Stimus :type "AIStimulus Structure"))
  (if (not (`|EnumEquality` (`self.Stats`) "NewEnumerator2"))
    (`BlackboardComponent.SetValueAsVector` (`self.Blackboard Component`) "InvestigateLoc" Stimus_StimulusLocation)
    (`BlackboardComponent.SetValueAsEnum` (`self.Blackboard Component`) "Stat" (enumliteral `/Game/Tank/AI/Enum/E_Stats` "NewEnumerator1"))))

(fn `On See`
  (params (Sitimus :type "AIStimulus Structure"))
  (`BlackboardComponent.SetValueAsEnum` (`self.Blackboard Component`) "Stat" (enumliteral `/Game/Tank/AI/Enum/E_Stats` "NewEnumerator2")))

(fn `UserConstructionScript`)