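; BP_Pawn is a player-controlled tank pawn with a mouse-aimed turret that fires rockets.
; BeginPlay adds the IMC_Tank Enhanced Input context and shows the cursor; input actions move along the base's right vector, yaw the base and spawn BP_Rocket at RocketSpawn.
; Each tick, a trace under the cursor sets the turret's world yaw, offset by -90 degrees and independent of base rotation.
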(event `self.ReceiveBeginPlay`
  (bind _asplayer_controller (cast `PlayerController` (`self.GetController`)))
  (`EnhancedInputSubsystemInterface.AddMappingContext` (pcsubsystem `EnhancedInputLocalPlayerSubsystem` _asplayer_controller) "/Game/Tank/MyChar/input/IMC_Tank.IMC_Tank" 0 (struct))
  (set `PlayerController.bShowMouseCursor` true (`GameplayStatics.GetPlayerController` 0)))

(event `EnhancedInput|/Game/Tank/MyChar/input/IA_LR`
  (params (ActionValue :type "Float (double-precision)") (ElapsedSeconds :type "Float (double-precision)") (TriggeredSeconds :type "Float (double-precision)") (InputAction :type "InputAction Object Reference" :default "/Game/Tank/MyChar/input/IA_LR.IA_LR"))
  (:`Triggered`
    (`SceneComponent.K2_AddWorldRotation` (`self.Base`) (`KismetMathLibrary.MakeRotator` 0.0 0.0 ActionValue) false false)))

(event `EnhancedInput|/Game/Tank/MyChar/input/IA_FB`
  (params (ActionValue :type "Float (double-precision)") (ElapsedSeconds :type "Float (double-precision)") (TriggeredSeconds :type "Float (double-precision)") (InputAction :type "InputAction Object Reference" :default "/Game/Tank/MyChar/input/IA_FB.IA_FB"))
  (:`Triggered`
    (`self.AddMovementInput` (`SceneComponent.GetRightVector` (`self.BASE`)) ActionValue)))

(event `EnhancedInput|/Game/Tank/MyChar/input/IA_Fire`
  (params (ActionValue :type Boolean) (ElapsedSeconds :type "Float (double-precision)") (TriggeredSeconds :type "Float (double-precision)") (InputAction :type "InputAction Object Reference" :default "/Game/Tank/MyChar/input/IA_Fire.IA_Fire"))
  (:`Started`
    (`|SpawnActorFromClass` "/Game/Tank/Rocket/BP_Rocket.BP_Rocket_C" (`SceneComponent.K2_GetComponentToWorld` (`self.Rocket Spawn`)) "Undefined" "MultiplyWithRoot" null null)))

(event `self.ReceiveTick`
  (params (DeltaSeconds :type "Float (single-precision)"))
  (bind (_returnvalue_roll _returnvalue_pitch _returnvalue_yaw) (`KismetMathLibrary.BreakRotator` (`KismetMathLibrary.FindLookAtRotation` (`SceneComponent.K2_GetComponentLocation` (`self.Turret`)) (`.Location` (`GameplayStatics.BreakHitResult` (`PlayerController.GetHitResultUnderCursorByChannel` (`GameplayStatics.GetPlayerController` 0) "TraceTypeQuery1" true))))))
  (`SceneComponent.K2_SetWorldRotation` (`self.Turret`) (`KismetMathLibrary.MakeRotator` 0.0 0.0 (+ _returnvalue_yaw -90.0)) false false))

(fn `UserConstructionScript`)